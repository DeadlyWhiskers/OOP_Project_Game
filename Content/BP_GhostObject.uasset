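; Ghost actor Blueprint that handles hit and death reactions on its movement component and sprite.
; UpdateHP briefly slows movement and tints the sprite red in parallel sequence branches, each restored after a short delay.
; OnDeath sets the Pomer flag, stops movement and destroys the actor after one second.
; The flag keeps a pending hit slowdown from restoring speed on a dead ghost.
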(event EventBeginPlay)

(event Collision|EventActorBeginOverlap
  (params (OtherActor :type Actor%20Object%20Reference)))

(event EventTick
  (params (DeltaSeconds :type Float%20%28single-precision%29)))

(event EventOnDeath
  (Variables|Default|SetPomer true)
  (Variables|/Script/Engine.FloatingPawnMovement|SetMaxSpeed (Variables|Default|GetMovement) 0.0)
  (Utilities|FlowControl|Delay 1.0)
  (Actor|DestroyActor))

(event EventUpdateHP
  (bind _movement (Variables|Default|GetMovement))
  (bind _sprite (Variables|Default|GetSprite))
  (Utilities|FlowControl|Sequence
    (:then_0
      (Variables|/Script/Engine.FloatingPawnMovement|SetMaxSpeed _movement 2e+01)
      (Utilities|FlowControl|Delay 0.2)
      (if (not (Variables|Default|GetPomer))
        (Variables|/Script/Engine.FloatingPawnMovement|SetMaxSpeed _movement 1e+02)))
    (:then_1
      (Sprite|SetSpriteColor _sprite "(R=1.000000,G=0.000000,B=0.000000,A=1.000000)")
      (Utilities|FlowControl|Delay 0.2)
      (Sprite|SetSpriteColor _sprite "(R=1.000000,G=1.000000,B=1.000000,A=1.000000)"))))

(fn ConstructionScript)