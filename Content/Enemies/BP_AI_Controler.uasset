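; Enemy AI controller that makes its controlled pawn chase the player.
; Every Tick it issues a new MoveToLocation request to the current location of player pawn 0.
; Unconnected leftover nodes hold experiments with MoveToActor, random reachable points and direct movement input on a BP_Fish pawn, none of which run.
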(event EventBeginPlay)

(event EventTick
  (params (DeltaSeconds :type Float%20%28single-precision%29))
  (AI|Navigation|MovetoLocation (Transformation|GetActorLocation (Game|Player|GetPlayerPawn 0)) -1.0 true true false true 0))

(fn ConstructionScript)