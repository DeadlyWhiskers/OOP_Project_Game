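; BP_Door is a door actor that shifts the player pawn's camera as the player passes through its trigger volumes.
; Box1 and Box2 each respond to a BP_PlayerPawn overlap by passing the location of their matching marker, Cube1 or Cube2, to SetCameraLocation.
; A distance check, using only the camera's X and Y against the marker's location, skips the move within a small threshold.
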(event OnComponentBeginOverlap(Box1)
  (params (OverlappedComponent :type Primitive%20Component%20Object%20Reference) (OtherActor :type Actor%20Object%20Reference) (OtherComp :type Primitive%20Component%20Object%20Reference) (OtherBodyIndex :type Integer) (bFromSweep :type Boolean) (SweepResult :type Hit%20Result%20Structure%20%28by%20ref%29))
  (bind _cube_1 (Variables|Default|GetCube%201))
  (bind _returnvalue (Transformation|GetWorldLocation _cube_1))
  (bind _asbp_player_pawn (Utilities|Casting|CastToBP_PlayerPawn OtherActor))
  (if (> (Math|Vector|Distance(Vector) (Math|Vector|MakeVector (.x (Transformation|GetWorldLocation (Variables|/Script/OOP_Project_Game.CC_PlayerClass|GetCamera _asbp_player_pawn))) (.y (Transformation|GetWorldLocation (Variables|/Script/OOP_Project_Game.CC_PlayerClass|GetCamera _asbp_player_pawn))) 0.0) _returnvalue) 2e+01)
    (Class|CCPlayerClass|SetCameraLocation _asbp_player_pawn _returnvalue)))

(event OnComponentBeginOverlap(Box2)
  (params (OverlappedComponent :type Primitive%20Component%20Object%20Reference) (OtherActor :type Actor%20Object%20Reference) (OtherComp :type Primitive%20Component%20Object%20Reference) (OtherBodyIndex :type Integer) (bFromSweep :type Boolean) (SweepResult :type Hit%20Result%20Structure%20%28by%20ref%29))
  (bind _cube_2 (Variables|Default|GetCube%202))
  (bind _returnvalue (Transformation|GetWorldLocation _cube_2))
  (bind _asbp_player_pawn (Utilities|Casting|CastToBP_PlayerPawn OtherActor))
  (if (> (Math|Vector|Distance(Vector) (Math|Vector|MakeVector (.x (Transformation|GetWorldLocation (Variables|/Script/OOP_Project_Game.CC_PlayerClass|GetCamera _asbp_player_pawn))) (.y (Transformation|GetWorldLocation (Variables|/Script/OOP_Project_Game.CC_PlayerClass|GetCamera _asbp_player_pawn))) 0.0) _returnvalue) 2e+01)
    (Class|CCPlayerClass|SetCameraLocation _asbp_player_pawn _returnvalue)))

(event EventBeginPlay)

(event Collision|EventActorBeginOverlap
  (params (OtherActor :type Actor%20Object%20Reference)))

(event EventTick
  (params (DeltaSeconds :type Float%20%28single-precision%29)))

(fn ConstructionScript)