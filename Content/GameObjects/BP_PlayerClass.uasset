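; Player Blueprint that handles the on-screen HUD and a custom crosshair cursor.
; BeginPlay creates both widgets and adds them to the viewport, then Tick moves the crosshair to the platform mouse position with DPI scale removed.
; Reload progress, weapon switch and HP events each forward to a matching update call for reload, weapon or health.
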(event EventBeginPlay
  (bind _returnvalue (UserInterface|CreateWidget "/Game/HUD/HUD_WIdget.HUD_WIdget_C"))
  (UserInterface|Viewport|AddtoViewport _returnvalue 0)
  (Variables|Default|SetHud _returnvalue)
  (bind _returnvalue_2 (UserInterface|CreateWidget "/Game/HUD/CS_RedAim_Crosshairs.CS_RedAim_Crosshairs_C"))
  (bind _output_get (Variables|Default|SetCursor _returnvalue_2))
  (UserInterface|Viewport|AddtoViewport _output_get 0))

(event Collision|EventActorBeginOverlap
  (params (OtherActor :type Actor%20Object%20Reference)))

(event EventTick
  (params (DeltaSeconds :type Float%20%28single-precision%29))
  (bind _returnvalue (Class|WidgetLayoutLibrary|GetMousePositiononPlatform))
  (Class|UserWidget|SetPositioninViewport (Variables|Default|GetCursor) _returnvalue true))

(event EventUpdateReloadProgress
  (Default|CallUpdateReload))

(event EventOnWeaponSwitch
  (Default|CallUpdateWeapon))

(event EventUpdateHP
  (Default|CallUpdateHealth))

(fn ConstructionScript)