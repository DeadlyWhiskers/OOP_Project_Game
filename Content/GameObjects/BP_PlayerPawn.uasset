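; Player pawn Blueprint that creates the player's HUD and relays gameplay state changes for display updates.
; On BeginPlay it creates the HUD widget, adds it to the viewport and stores the reference.
; Events for reload progress, weapon switch, HP and shooting each fire a matching update dispatcher, rather than calling the widget directly.
; It holds no movement or combat logic, and its Tick, overlap and construction script are empty.
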(event EventBeginPlay
  (bind _returnvalue (UserInterface|CreateWidget "/Game/HUD/HUD_WIdget.HUD_WIdget_C"))
  (UserInterface|Viewport|AddtoViewport _returnvalue 0)
  (Variables|Default|SetHUD _returnvalue))

(event Collision|EventActorBeginOverlap
  (params (OtherActor :type Actor%20Object%20Reference)))

(event EventOnShoot
  (Default|CallUpdateShootProgressBar))

(event EventUpdateReloadProgress
  (Default|CallUpdateReload))

(event EventOnWeaponSwitch
  (Default|CallUpdateWeapon))

(event EventUpdateHP
  (Default|CallUpdateHealth))

(event EventTick
  (params (DeltaSeconds :type Float%20%28single-precision%29)))

(fn ConstructionScript)